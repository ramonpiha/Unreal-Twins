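; SensorDataPolling is an actor Blueprint that polls an HTTP endpoint for sensor readings and logs the polling latency.
; StartApiPolling starts a looping five-second timer that sends a GET request and extracts the JSON field named by SensorType.
; The "on" type fills ButtonValue, while other types fill ReturnValue.
; Each successful response appends round-trip milliseconds and ReturnValue to a CSV at a hardcoded local thesis path.
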(event `StartApiPolling`
  (`KismetSystemLibrary.K2_SetTimerDelegate` (delegate `ApiPolling`) 5.0 true))

(event `ApiPolling`
  (bind (_seconds _partialseconds) (`GameplayStatics.GetAccurateRealTime`))
  (bind (_seconds_2 _partialseconds_2) (`GameplayStatics.GetAccurateRealTime`))
  (bind _sensortype (`self.SensorType`))
  (set `self.StartTime` (`KismetMathLibrary.Conv_DoubleToInt64` (* (+ _seconds _partialseconds) 1000.0)))
  (bind (_outheader _result_body) (`|HttpRequest` (`self.endpoint`) "Get")
    (:`On Success`
      (if (`KismetStringLibrary.EqualEqual_StrStr` _sensortype "on")
        (bind _outvalue (`|GetJsonField` _result_body _sensortype))
        (set `self.ButtonValue` _outvalue)
        (else
          (bind _outvalue_2 (`|GetJsonField` _result_body _sensortype))
          (bind _output_get (set `self.ReturnValue` _outvalue_2))))
      (`VictoryBPFunctionLibrary.FileIO__SaveStringTextToFile` "C:\\Users\\ramon\\Documents\\School\\Master\\MasterThesis" "DataPollingTime.csv" (`KismetStringLibrary.Concat_StrStr` (`KismetStringLibrary.Conv_Int64ToString` (- (* (+ _seconds_2 _partialseconds_2) 1000.0) (`self.StartTime`))) "," (`KismetStringLibrary.Conv_IntToString` _output_get)) true true))))

(fn `UserConstructionScript`)